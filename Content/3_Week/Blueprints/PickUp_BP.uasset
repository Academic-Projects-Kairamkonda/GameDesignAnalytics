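; Coin pickup actor that adds its Value to the player character's Score on overlap.
; On BeginPlay it writes Value to its CoinValue text so the worth of the coin is shown.
; When an overlapping actor casts to ThirdPersonCharacter, it increases that character's Score and destroys itself; other actors are ignored.
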(event `self.ReceiveBeginPlay`
  ;[1 1 1] Add coin value
  (`TextRenderComponent.K2_SetText` (`self.CoinValue`) (`KismetTextLibrary.Conv_IntToText` (`self.Value`))))

(event `self.ReceiveActorBeginOverlap`
  (params (OtherActor :type "Actor Object Reference"))
  (bind _asthird_person_character (cast `/Game/ThirdPersonBP/Blueprints/ThirdPersonCharacter` OtherActor))
  (set `/Game/ThirdPersonBP/Blueprints/ThirdPersonCharacter.Score` (+ (`/Game/ThirdPersonBP/Blueprints/ThirdPersonCharacter.Score` _asthird_person_character) (`self.Value`)) _asthird_person_character)
  (`self.K2_DestroyActor`))

(fn `UserConstructionScript`)